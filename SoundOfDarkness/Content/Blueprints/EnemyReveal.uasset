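; EnemyReveal is an actor, by name an enemy reveal, that hides its root and children at BeginPlay.
; Begin and end overlaps with a circularExpansion-green actor feed one shared SetVisibility call on the root only, without propagating to children.
; Visibility is true only while the begin-overlap cast result is valid and the end-overlap one is not, so a stored end result keeps it hidden while valid.
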(event EventBeginPlay
  (Rendering|SetVisibility (Variables|Default|GetDefaultSceneRoot) false true))

(event Collision|EventActorBeginOverlap
  (params (OtherActor :type Actor%20Object%20Reference))
  (bind _ascircular_expansion_green (Utilities|Casting|CastTocircularExpansion-green OtherActor))
  (Rendering|SetVisibility (Variables|Default|GetDefaultSceneRoot) (and (not (Utilities|IsValid (stale Collision|EventActorEndOverlap _ascircular_expansion_green))) (Utilities|IsValid _ascircular_expansion_green)) false))

(event EventTick
  (params (DeltaSeconds :type Float%20%28single-precision%29)))

(event Collision|EventActorEndOverlap
  (params (OtherActor :type Actor%20Object%20Reference))
  (bind _ascircular_expansion_green (Utilities|Casting|CastTocircularExpansion-green OtherActor))
  (Rendering|SetVisibility (Variables|Default|GetDefaultSceneRoot) (and (not (Utilities|IsValid _ascircular_expansion_green)) (Utilities|IsValid (stale Collision|EventActorBeginOverlap _ascircular_expansion_green))) false))

(fn ConstructionScript)