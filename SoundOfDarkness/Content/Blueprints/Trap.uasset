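; A Paper2D trap actor that springs when a player walks into it and triggers that character's death.
; On overlap with an actor tagged Player, it plays the trap flipbook once and fires the Trap sound event at its own location.
; After a short delay it casts the overlapping actor to 2DSideScrollerCharacter and calls IsDead, without rechecking that it still overlaps.
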(event EventBeginPlay)

(event EventTick
  (params (DeltaSeconds :type Float%20%28single-precision%29)))

(event Collision|EventActorBeginOverlap
  (params (OtherActor :type Actor%20Object%20Reference))
  (bind _sprite (Variables|Default|GetSprite))
  (if (Actor|ActorHasTag OtherActor "Player")
    (Components|Timeline|SetLooping _sprite false)
    (Sprite|SetFlipbook _sprite "/Game/2DSideScroller/FlipBooks/TrapAnim.TrapAnim")
    (Class|FMODBlueprintStatics|PlayEventatLocation "/Game/FMOD/Events/Environment/Trap.Trap" (Math|Conversions|ToTransform(Vector) (Transformation|GetActorLocation)))
    (Utilities|FlowControl|Delay 0.5)
    (bind _as2dside_scroller_character (Utilities|Casting|CastTo2DSideScrollerCharacter OtherActor))
    (Default|IsDead _as2dside_scroller_character)))

(fn ConstructionScript)